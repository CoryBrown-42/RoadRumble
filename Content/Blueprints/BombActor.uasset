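; Bomb actor that explodes when its sphere is overlapped and damages BattleCarsPawn vehicles.
; The overlap runs on authority and calls Explode, noted as a multicast.
; Explode hides the mesh, plays sound, fires a radial impulse, spawns a random explosion emitter, then destroys the actor after a delay.
; Pawn hits pass a DoOnce and apply GE_Damage through the Ability System; other actors trigger only the explosion, bypassing that guard.
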(event OnComponentBeginOverlap(Sphere)
  (params (OverlappedComponent :type Primitive%20Component%20Object%20Reference) (OtherActor :type Actor%20Object%20Reference) (OtherComp :type Primitive%20Component%20Object%20Reference) (OtherBodyIndex :type Integer) (bFromSweep :type Boolean) (SweepResult :type Hit%20Result%20Structure%20%28by%20ref%29))
  ;[1 1 1] On Overlap call Explode Multi-Cast
  (Networking|SwitchHasAuthority
    (:Authority
      (CallFunction|Explode OtherActor))))

(event Custom|Explode
  (params (HitActor :type Actor%20Object%20Reference))
  (bind _explosions (Variables|Default|GetExplosions))
  (bind _staticmeshcomponent (Variables|Default|GetStaticMeshComponent))
  (bind _returnvalue (Transformation|GetWorldLocation _staticmeshcomponent))
  ;[1 1 1] Explosion
  (bind _asbattle_cars_pawn (Utilities|Casting|CastToBattleCarsPawn HitActor)
    (:then
      (Utilities|FlowControl|DoOnce false
        (:Completed
          (Development|PrintString "Damage")
          (Utilities|FlowControl|Sequence
            (:then_0
              (Development|SetHiddeninGame (Variables|Default|GetStaticMeshComponent) true false :!label _label)
              (Audio|PlaySoundatLocation "/Game/Sounds/Explosions/zapsplat_explosion_fireball_43738_01_Cue.zapsplat_explosion_fireball_43738_01_Cue" _returnvalue "0, 0, 0" 1.0 1.0 0.0 "/Game/BallisticsVFX/SFX/Attentuations/ImpactsAttenuation.ImpactsAttenuation" 0 0)
              (Class|RadialForceComponent|FireImpulse (Variables|Default|GetRadialForce))
              (Effects|SpawnEmitteratLocation (Utilities|Array|Get(acopy) _explosions (Math|Random|RandomIntegerinRange 0 (- (Utilities|Array|Length _explosions) 1))) _returnvalue (Math|Rotator|MakeRotator 0.0 0.0 (Math|Random|RandomFloatinRange 0.0 3.6e+02)))
              (Utilities|FlowControl|Delay 2.0)
              (Actor|DestroyActor))
            (:then_1
              (GameplayEffects|ApplyGameplayEffectToSelf :self (Variables|/Script/BattleCars.BattleCarsPawn|GetAbilitySystemComponent _asbattle_cars_pawn) :GameplayEffectClass "/Game/Abilities/GE_Damage.GE_Damage_C" :Level 1.0))))))
    (:CastFailed
      (goto _label))))

(event EventBeginPlay
  ;[1 1 1] Explosion
  (|CallParentFunction) ; This node is disabled and will not be called.\nDrag off pins to build functionality.
)

(event EventTick
  (params (DeltaSeconds :type Float%20%28single-precision%29))
  (|CallParentFunction DeltaSeconds) ; This node is disabled and will not be called.\nDrag off pins to build functionality.
)

(fn ConstructionScript
  (|CallParentFunction))