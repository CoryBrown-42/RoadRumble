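; TimeDilation is an item actor that alters the time rate of a vehicle based on its distance from the actor.
; Overlap stores any BP_BaseVehiclePawn as Player, and nothing clears that reference afterwards.
; Each Tick sets that pawn's CustomTimeDilation from clamped distance and prints it for debugging.
; The Lerp alpha is effectively raw distance, so dilation grows roughly quadratically, from near-frozen at the center to far above normal speed.
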(event Collision|EventActorBeginOverlap
  (params (OtherActor :type Actor%20Object%20Reference))
  (bind _asbp_base_vehicle_pawn (Utilities|Casting|CastToBP_BaseVehiclePawn OtherActor))
  (Variables|Default|SetPlayer _asbp_base_vehicle_pawn))

(event EventTick
  (params (DeltaSeconds :type Float%20%28single-precision%29))
  (bind _player (Variables|Default|GetPlayer)
    (:then
      (Variables|/Script/Engine.Actor|SetCustomTimeDilation _player (Math|Float|Lerp 0.001 (/ (Math|Float|Clamp(Float) (Transformation|GetDistanceTo _player self) 0.001 1e+03) 1e+02) (Math|Float|NormalizetoRange (Math|Float|Clamp(Float) (Transformation|GetDistanceTo _player self) 0.001 1e+03) 0.0 1.0)))
      (Development|PrintString (Utilities|String|ToString(Float) (Variables|/Script/Engine.Actor|GetCustomTimeDilation (Variables|Default|GetPlayer)))))
    (:else)))

(fn ConstructionScript)