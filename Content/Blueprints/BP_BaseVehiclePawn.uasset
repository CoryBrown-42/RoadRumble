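; Base vehicle pawn that fires a weapon on Shoot input and drives an engine sound parameter from forward velocity.
; Attack uses a predicted projectile path as an instant hit test, applying GAS damage to vehicle pawns, exploding bombs and pushing physics bodies.
; PlayFX spawns particles, sound and decals by surface type at muzzle and impact.
; Debug drawing remains active; AttackClient and MoveMeshAlongPath are empty stubs.
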(event Custom|Attack
  (bind _firepoint (Variables|Default|GetFirePoint))
  (bind _returnvalue (Transformation|GetWorldLocation _firepoint))
  (bind _returnvalue_2 (Math|Vector|GetForwardVector _firepoint))
  (CallFunction|PlayFX (Collision|MakeHitResult true false 0.0 0.0 _returnvalue "0, 0, 0" "0,0,1" _returnvalue_2 "/Game/Physics/Plastic.Plastic" self))
  (bind (_outhit _outpathpositions) (Class|GameplayStatics|BlueprintPredictProjectilePathbyObjectType _returnvalue (* _returnvalue_2 6e+04) true 2e+01 (Utilities|Array|MakeArray "ObjectTypeQuery3" "ObjectTypeQuery4" "ObjectTypeQuery5" "ObjectTypeQuery2" "ObjectTypeQuery1") true (Utilities|Array|MakeArray self) "ForOneFrame" 1e+01 1.0 0.5 -69.0))
  (CallFunction|MoveMeshAlongPath _outpathpositions)
  (if (.bBlockingHit (Collision|BreakHitResult _outhit))
    (Utilities|FlowControl|Sequence
      (:then_0
        ;[1 1 1] Apply Hit Gameplay ability.
        (bind _asbp_base_vehicle_pawn (Utilities|Casting|CastToBP_BaseVehiclePawn (.HitActor (Collision|BreakHitResult _outhit))))
        (GameplayEffects|ApplyGameplayEffectToSelf :self (Variables|/Script/BattleCars.BattleCarsPawn|GetAbilitySystemComponent _asbp_base_vehicle_pawn) :GameplayEffectClass "/Game/Abilities/GE_Damage.GE_Damage_C" :Level 1.0)
        (CallFunction|TakeDamage (.Location (Collision|BreakHitResult _outhit))))
      (:then_1
        ;[1 1 1] IF hit Bomb
        (bind _asbomb_actor (Utilities|Casting|CastToBombActor (.HitActor (Collision|BreakHitResult _outhit))))
        (Default|Explode _asbomb_actor _asbomb_actor))
      (:then_2
        ;[1 1 1] If simulating physics Add Radial Impulse
        (if (Physics|IsSimulatingPhysics (.HitComponent (Collision|BreakHitResult _outhit)) "None")
          (Physics|AddRadialImpulse (.HitComponent (Collision|BreakHitResult _outhit)) (.Location (Collision|BreakHitResult _outhit)) 666.0 (Variables|Default|GetImpulseIntensity) "RIF_Constant" true)))
      (:then_3
        (CallFunction|PlayFX _outhit)))))

(event Custom|AttackClient)

(event Custom|TakeDamage
  (params (Center :type Vector))
  (Rendering|Debug|DrawDebugCircle Center 2e+01 12 "(R=1.000000,G=0.044383,B=0.000000,A=1.000000)" 2e+01 2e+01 "0.000000,1.000000,0.000000" "0.000000,0.000000,1.000000" true)
  (Class|VisualLoggerKismetLibrary|LogText 0 "GAS Hit" "VisLogBP"))

(event EventBeginPlay)

(event EventTick
  (params (DeltaSeconds :type Float%20%28single-precision%29))
  (Audio|Parameter|SetFloatParameter (Variables|Default|GetEngineSounds) "Speed" (Math|Float|NormalizetoRange (Math|Vector|DotProduct (Variables|/Script/Engine.MovementComponent|GetVelocity (Variables|Default|GetVehicleMovement)) (Math|Vector|GetForwardVector (Variables|Character|GetMesh))) 0.0 1.0) :!class /Script/Engine.AudioComponent))

(event Input|ActionEvents|InputActionShoot
  (params (Key :type Key%20Structure))
  ;[1 1 1] Attack Input
  (:Pressed
    (CallFunction|Attack)
    (CallFunction|AttackCLient)))

(event Input|AxisEvents|InputAxisShoot
  (params (AxisValue :type Float%20%28single-precision%29)))

(event Input|MouseEvents|LeftMouseButton
  (params (Key :type Key%20Structure)))

(event Input|KeyboardEvents|V
  (params (Key :type Key%20Structure)))

(fn ConstructionScript
  (Rendering|Material|SetScalarParameterValue "/Game/Materials/GlobalMatParams.GlobalMatParams" "Mask" (Variables|Default|GetMask) :!class /Script/Engine.KismetMaterialLibrary))

(fn MoveMeshAlongPath
  (params (Array :type Array%20of%20Vectors))
  (for _array_element Array
    _))

(fn PlayFX
  (params (Hit :type Hit%20Result%20Structure%20%28by%20ref%29))
  (bind (_bblockinghit _binitialoverlap _time _distance _location _impactpoint _normal _impactnormal _physmat _hitactor _hitcomponent) (Collision|BreakHitResult Hit))
  (bind _returnvalue (Math|Rotator|MakeRotfromZX _impactnormal _normal))
  (Utilities|FlowControl|Sequence
    (:then_0
      (switch Utilities|FlowControl|Switch|SwitchonEPhysicalSurface (Collision|GetSurfaceType Hit)
        (:SurfaceType_Default
          ;[1 1 1] Default currently plastic - change later
          (LocalVariables|SetParticleSystem "/Game/AdvancedMagicFX13/Particles/P_ky_impact.P_ky_impact")
          (LocalVariables|SetSound "/Game/BallisticsVFX/SFX/Guns/HiPowered.HiPowered")
          (LocalVariables|SetDecal "/Game/BallisticsVFX/Decals/Decals__Ricochet_Gen2.Decals__Ricochet_Gen2"))
        (:SurfaceType1
          (LocalVariables|SetParticleSystem "/Game/BallisticsVFX/Particles/Impacts/DynamicImpacts/Plastic/Plastic_impact_Dyn.Plastic_impact_Dyn")
          (LocalVariables|SetSound "/Game/BallisticsVFX/SFX/Impacts/PolySnaps_Impacts.PolySnaps_Impacts")
          (LocalVariables|SetDecal "/Game/BallisticsVFX/Decals/Decals_Plastic.Decals_Plastic"))
        (:SurfaceType2
          (LocalVariables|SetParticleSystem "/Game/VFX_Toolkit_V1/ParticleSystems/356Days/Par_WildImpact_01.Par_WildImpact_01")
          (LocalVariables|SetSound "/Game/BallisticsVFX/SFX/Impacts/Metal_Dull_Impacts.Metal_Dull_Impacts")
          (LocalVariables|SetDecal "/Game/BallisticsVFX/Decals/Decals_Metal.Decals_Metal"))
        (:SurfaceType3
          (LocalVariables|SetParticleSystem "/Game/BallisticsVFX/Particles/Impacts/DynamicImpacts/Grass/Grass_impact_Dyn.Grass_impact_Dyn")
          (LocalVariables|SetSound "/Game/BallisticsVFX/SFX/Impacts/Dirt_Impacts.Dirt_Impacts")
          (LocalVariables|SetDecal "/Game/BallisticsVFX/Decals/Decals_Soil.Decals_Soil"))))
    (:then_1
      (Effects|SpawnEmitteratLocation (LocalVariables|GetParticleSystem) _location _returnvalue "1.000000,1.000000,1.000000" false "AutoRelease")
      (Audio|PlaySoundatLocation (LocalVariables|GetSound) _location "0, 0, 0" 1.0 1.0 0.0 "/Game/BallisticsVFX/SFX/Attentuations/ImpactsAttenuation.ImpactsAttenuation" 0 0)
      (Rendering|Debug|DrawDebugSphere _location 1e+02 12 "(R=20.000000,G=0.000000,B=0.565720,A=1.000000)" 1e+01 2.0)
      (Rendering|Decal|SpawnDecalatLocation 0 "20.000000,20.000000,20.000000" _location _returnvalue 25.0))))